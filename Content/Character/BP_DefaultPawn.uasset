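; Default pawn Blueprint that feeds its health and nickname into an MVVM character stat view model held by the game mode.
; On BeginPlay it binds the HP and nickname component change delegates, then initializes the view model with current values.
; Each change event writes the new value straight into that view model.
; Pressing Space sets max HP to a fixed value, apparently as a test of the binding.
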(event `OnHpChange_Event`
  (params (CurrentHp :type "Float (single-precision)"))
  (set `/Game/UI/BPVM_CharacterStat.CurrentHp` CurrentHp (`/Game/Game/BP_MVVMGameMode.BPVMCharacterStat` (stale `self.ReceiveBeginPlay` _asbp_mvvmgame_mode))))

(event `OnMaxHpChange_Event`
  (params (MaxHp :type "Float (single-precision)"))
  (set `/Game/UI/BPVM_CharacterStat.MaxHp` MaxHp (`/Game/Game/BP_MVVMGameMode.BPVMCharacterStat` (stale `self.ReceiveBeginPlay` _asbp_mvvmgame_mode))))

(event `OnNicknameChanged_Event`
  (params (InNickname :type String))
  (set `/Game/UI/BPVM_CharacterStat.NickName` (`KismetTextLibrary.Conv_StringToText` InNickname) (`/Game/Game/BP_MVVMGameMode.BPVMCharacterStat` (stale `self.ReceiveBeginPlay` _asbp_mvvmgame_mode))))

(event `self.ReceiveBeginPlay`
  (bind _asbp_mvvmgame_mode (cast `/Game/Game/BP_MVVMGameMode` (`GameplayStatics.GetGameMode`)))
  (`|ExecutionSequence`
    (:`then_0`
      (bind _returnvalue (`self.GetHpComponent`))
      (add `HpComponent.OnHpChange` _returnvalue (delegate `OnHpChange_Event`))
      (add `HpComponent.OnMaxHpChange` _returnvalue (delegate `OnMaxHpChange_Event`)))
    (:`then_1`
      (bind _returnvalue_2 (`self.GetNicknameComponent`))
      (add `NicknameComponent.OnNicknameChanged` _returnvalue_2 (delegate `OnNicknameChanged_Event`)))
    (:`then_2`
      (`/Game/UI/BPVM_CharacterStat.IntitViewModel` (`/Game/Game/BP_MVVMGameMode.BPVMCharacterStat` _asbp_mvvmgame_mode) (`HpComponent.GetHp` _returnvalue) (`HpComponent.GetMaxHp` _returnvalue) (`NicknameComponent.GetNickname` _returnvalue_2)))))

(event `Key|SpaceBar`
  (params (Key :type "Key Structure"))
  (:`Pressed`
    (bind _returnvalue (`self.GetHpComponent`))
    (`HpComponent.SetMaxHp` _returnvalue 200.0)))

(fn `UserConstructionScript`)